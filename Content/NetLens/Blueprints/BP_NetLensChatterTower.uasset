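; BP_NetLensChatterTower is a NetLens tower actor with a spinning dish, apparently built to produce steady network chatter.
; Tick yaws the dish on every machine at a constant rate derived from game time.
; With authority, it also writes SweepAngle from the same formula and a PingCounter that increments several times a second.
; TowerPing is an empty event that nothing in this graph calls.
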(event `self.ReceiveTick`
  (params (DeltaSeconds :type "Float (single-precision)"))
  (bind _returnvalue (`KismetSystemLibrary.GetGameTimeInSeconds`))
  (`SceneComponent.K2_SetRelativeRotation` (`self.Dish`) (`KismetMathLibrary.MakeRotator` 0.0 0.0 (* _returnvalue 55.0)) false false)
  (if (`self.HasAuthority` self)
    (set `self.SweepAngle` (* _returnvalue 55.0))
    (set `self.PingCounter` (`KismetMathLibrary.FTrunc` (* _returnvalue 4.0)))))

(event `TowerPing`)

(fn `UserConstructionScript`)