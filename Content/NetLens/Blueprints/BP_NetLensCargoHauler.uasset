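; NetLens cargo hauler actor that generates continuously changing ship state on the server while flying a looping route.
; BeginPlay seeds a twelve-berth crew roster, hull integrity and an idle manifest code, on authority only.
; An authority-only Tick uses offset game time to drive sine-based throttle, hull, bay doors and docking target, plus manifest text and two roster entries.
; The same clock moves the actor along a figure-eight Lissajous path with steadily spinning yaw.
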(event `self.ReceiveBeginPlay`
  (if (`self.HasAuthority` self)
    (`KismetArrayLibrary.Array_Clear` (`self.CrewRoster`))
    (for _index (range 12)
      (`KismetArrayLibrary.Array_Add` (`self.CrewRoster`) (`KismetStringLibrary.Concat_StrStr` "Crew-Berth-" (`KismetStringLibrary.Conv_IntToString` _index))))
    (set `self.HullIntegrity` 1.0)
    (set `self.ManifestCode` "MANIFEST-IDLE")))

(event `self.ReceiveTick`
  (params (DeltaSeconds :type "Float (single-precision)"))
  (bind _routeradius (`self.RouteRadius`))
  (bind _returnvalue (+ (`KismetSystemLibrary.GetGameTimeInSeconds`) (`self.RouteOffset`)))
  (if (`self.HasAuthority` self)
    (set `self.Phase` _returnvalue)
    (set `self.Throttle` (`KismetMathLibrary.DegSin` (* _returnvalue 40.0)))
    (set `self.HullIntegrity` (+ 0.5 (* 0.5 (`KismetMathLibrary.DegCos` (* _returnvalue 25.0)))))
    (set `self.BayDoorsOpen` (> (`KismetMathLibrary.DegSin` (* _returnvalue 30.0)) 0.0))
    (set `self.DockingTarget` (`KismetMathLibrary.MakeVector` (* 1200.0 (`KismetMathLibrary.DegCos` (* _returnvalue 18.0))) (* 1200.0 (`KismetMathLibrary.DegSin` (* _returnvalue 18.0))) 520.0))
    (set `self.ManifestCode` (`KismetStringLibrary.Concat_StrStr` "MANIFEST-" (`KismetStringLibrary.Conv_DoubleToString` _returnvalue)))
    (`KismetArrayLibrary.Array_Set` (`self.CrewRoster`) 0 (`KismetStringLibrary.Concat_StrStr` "Watch-Officer-" (`KismetStringLibrary.Conv_DoubleToString` _returnvalue)))
    (`KismetArrayLibrary.Array_Set` (`self.CrewRoster`) 1 (`KismetStringLibrary.Concat_StrStr` "Loadmaster-" (`KismetStringLibrary.Conv_DoubleToString` (* _returnvalue 2.0))))
    (`self.K2_SetActorLocationAndRotation` self (`KismetMathLibrary.MakeVector` (* _routeradius (`KismetMathLibrary.DegCos` (* _returnvalue 11.0))) (* (* _routeradius 0.7) (`KismetMathLibrary.DegSin` (* _returnvalue 22.0))) 820.0) (`KismetMathLibrary.MakeRotator` 0.0 0.0 (* _returnvalue 11.0)) false false)))

(fn `UserConstructionScript`)