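; BP_NetLensDrone is a drone actor that circles the world origin while bobbing vertically.
; BeginPlay randomizes its orbit phase, radius, speed, lane height and route index on every instance, and turns the beacon flag on.
; On authority only, Tick computes position and tangent yaw from game time with sine/cosine, and oscillates CargoLevel.
; RouteIndex and BeaconOn are set but never read in these graphs.
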(event `self.ReceiveBeginPlay`
  (set `self.OrbitPhase` (`KismetMathLibrary.RandomFloatInRange` 0.0 360.0))
  (set `self.OrbitRadius` (`KismetMathLibrary.RandomFloatInRange` 550.0 2700.0))
  (set `self.OrbitSpeed` (`KismetMathLibrary.RandomFloatInRange` 10.0 44.0))
  (set `self.LaneHeight` (`KismetMathLibrary.RandomFloatInRange` 260.0 2500.0))
  (set `self.RouteIndex` (`KismetMathLibrary.RandomIntegerInRange` 0 11))
  (set `self.BeaconOn` true))

(event `self.ReceiveTick`
  (params (DeltaSeconds :type "Float (single-precision)"))
  (bind _returnvalue (`KismetSystemLibrary.GetGameTimeInSeconds`))
  (bind _orbitradius (`self.OrbitRadius`))
  (bind _returnvalue_2 (+ (`self.OrbitPhase`) (* _returnvalue (`self.OrbitSpeed`))))
  (if (`self.HasAuthority` self)
    (`self.K2_SetActorLocationAndRotation` self (`KismetMathLibrary.MakeVector` (* _orbitradius (`KismetMathLibrary.DegCos` _returnvalue_2)) (* _orbitradius (`KismetMathLibrary.DegSin` _returnvalue_2)) (+ (`self.LaneHeight`) (* 260.0 (`KismetMathLibrary.DegSin` (* _returnvalue 70.0))))) (`KismetMathLibrary.MakeRotator` 0.0 0.0 (+ _returnvalue_2 90.0)) false false)
    (set `self.CargoLevel` (`KismetMathLibrary.DegSin` (* _returnvalue 45.0)))))

(fn `UserConstructionScript`)