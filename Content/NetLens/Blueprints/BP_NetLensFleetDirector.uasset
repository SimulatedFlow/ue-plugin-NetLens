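; Fleet director actor that spawns a configurable number of BP_NetLensDrone actors when play begins.
; On BeginPlay, only the authority runs a loop that spawns DroneCount drones.
; All drones appear at the same point above the director with default rotation and scale, using AlwaysSpawn to ignore collisions.
; It keeps no references to the drones and has no further logic.
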(event `self.ReceiveBeginPlay`
  (if (`self.HasAuthority` self)
    (for _ (range (+ (- (`self.DroneCount`) 1) 1))
      (`|SpawnActorFromClass` "/NetLens/NetLens/Blueprints/BP_NetLensDrone.BP_NetLensDrone_C" (`KismetMathLibrary.MakeTransform` (+ (`self.K2_GetActorLocation` self) (`KismetMathLibrary.MakeVector` 0.0 0.0 500.0)) (`KismetMathLibrary.MakeRotator` 0.0) (`KismetMathLibrary.MakeVector` 1.0 1.0 1.0)) "AlwaysSpawn" "MultiplyWithRoot" null null))))

(fn `UserConstructionScript`)